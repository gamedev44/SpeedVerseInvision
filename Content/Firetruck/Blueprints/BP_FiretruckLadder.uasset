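; Drivable firetruck with a player-controlled ladder, working reverse lights and toggleable siren flash lights.
; Axis input drives the vehicle movement component and writes ladder rotation, clamped elevation and optional extension into the ladder AnimInstance.
; Ladder and flash-light changes pass through replication events that apply only on remote instances.
; Dummy colliders follow ladder sockets each tick because AnimBP-modified bones lack kinematic physics; lights use dynamic materials.
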(event `self.ReceiveBeginPlay`
  (bind _mesh (`self.Mesh`))
  (bind _assk_ladder_skeleton_anim_blueprint (cast `/Game/Firetruck/Meshes/SK_Ladder_Skeleton_AnimBlueprint` (`SkeletalMeshComponent.GetAnimInstance` (`self.LadderMesh`))))
  (set `self.AnimInstance` _assk_ladder_skeleton_anim_blueprint)
  (bind _returnvalue (`PrimitiveComponent.CreateDynamicMaterialInstance` _mesh 4 "/Game/Firetruck/Materials/M_Light.M_Light" "None"))
  (`MaterialInstanceDynamic.SetScalarParameterValue` _returnvalue "LightPower" 2000.0)
  (bind _returnvalue_2 (`PrimitiveComponent.CreateDynamicMaterialInstance` _mesh 5 "/Game/Firetruck/Materials/MI_Light_Rear.MI_Light_Rear" "None"))
  (`MaterialInstanceDynamic.SetScalarParameterValue` _returnvalue_2 "LightPower" 400.0)
  (bind _returnvalue_3 (`PrimitiveComponent.CreateDynamicMaterialInstance` (`self.Mesh`) 6 "/Game/Firetruck/Materials/MI_Light_Reverse.MI_Light_Reverse" "None"))
  (set `self.ReverseLight` _returnvalue_3))

(event `self.ReceiveTick`
  (params (DeltaSeconds :type "Float (single-precision)"))
  (bind _reverselight (`self.ReverseLight`))
  (bind _laddermesh (`self.LadderMesh`))
  (bind _returnvalue (`ChaosVehicleMovementComponent.GetCurrentGear` (`self.VehicleMovementComponent`)))
  (`|ExecutionSequence`
    (:`then_0`
      ;[1 1 1] Reverse lights
      (if (and (== (`self.SavedGear`) -1) (> _returnvalue 0))
        (`MaterialInstanceDynamic.SetScalarParameterValue` _reverselight "LightPower" 0.0)
        (elif (and (== _returnvalue -1) (!= (`self.SavedGear`) -1))
          (`MaterialInstanceDynamic.SetScalarParameterValue` _reverselight "LightPower" 250.0))))
    (:`then_1`
      (set `self.SavedGear` _returnvalue))
    (:`then_2`
      ;[1 1 1] Dummy collision for the ladder. When using TransformModifyBone in the AnimBP, kinematic physics do not work on the transforming bone.
      (`SceneComponent.K2_SetWorldTransform` (`self.LadderCollision1`) (`SceneComponent.GetSocketTransform` _laddermesh "ladder_002" "RTS_World") false false)
      (`SceneComponent.K2_SetWorldTransform` (`self.LadderCollision2`) (`SceneComponent.GetSocketTransform` _laddermesh "ladder_001" "RTS_World") false false))))

(event `InputAxis|MoveRight` :overrideparent false
  (params (AxisValue :type "Float (single-precision)"))
  ;[1 1 1] Steering input
  (`ChaosVehicleMovementComponent.SetSteeringInput` (`self.VehicleMovementComponent`) AxisValue))

(event `InputAxis|MoveForward` :overrideparent false
  (params (AxisValue :type "Float (single-precision)"))
  (bind _vehiclemovementcomponent (`self.VehicleMovementComponent`))
  ;[1 1 1] Throttle input
  (if (>= AxisValue 0.0)
    (`ChaosVehicleMovementComponent.SetThrottleInput` _vehiclemovementcomponent AxisValue)
    (`ChaosVehicleMovementComponent.SetBrakeInput` _vehiclemovementcomponent 0.0)
    (else
      (`ChaosVehicleMovementComponent.SetBrakeInput` _vehiclemovementcomponent (* AxisValue -1.0))
      (`ChaosVehicleMovementComponent.SetThrottleInput` _vehiclemovementcomponent 0.0))))

(event `InputAction|Handbrake`
  (params (Key :type "Key Structure"))
  (bind _vehiclemovementcomponent (`self.VehicleMovementComponent`))
  ;[1 1 1] Handbrake input
  (:`Pressed`
    (`ChaosVehicleMovementComponent.SetHandbrakeInput` _vehiclemovementcomponent true))
  (:`Released`
    (`ChaosVehicleMovementComponent.SetHandbrakeInput` _vehiclemovementcomponent false)))

(event `SetLateral`
  (params (NewParam :type "Rotator Structure"))
  (bind _animinstance (`self.AnimInstance`))
  ;[1 1 1] Replicated
  (`/Engine/EditorBlueprintResources/StandardMacros.IsValid` _animinstance
    (:`Is Valid`
      (`/Engine/EditorBlueprintResources/ActorMacros.Switch Has Authority`
        (:`Remote`
          (set `/Game/Firetruck/Meshes/SK_Ladder_Skeleton_AnimBlueprint.LadderLateral` NewParam _animinstance))))))

(event `InputAxis|LadderLateral`
  (params (AxisValue :type "Float (single-precision)"))
  (bind _animinstance (`self.AnimInstance`))
  ;[1 1 1] Ladder Movement
  (bind _output_get (set `/Game/Firetruck/Meshes/SK_Ladder_Skeleton_AnimBlueprint.LadderLateral` (`KismetMathLibrary.ComposeRotators` (`/Game/Firetruck/Meshes/SK_Ladder_Skeleton_AnimBlueprint.LadderLateral` _animinstance) (`KismetMathLibrary.MakeRotator` 0.0 0.0 (* (`GameplayStatics.GetWorldDeltaSeconds`) AxisValue 12.5))) _animinstance))
  (`self.SetLateral` _output_get))

(event `InputAxis|Turn`
  (params (AxisValue :type "Float (single-precision)"))
  ;[1 1 1] Turn
  (`self.AddControllerYawInput` AxisValue))

(event `InputAxis|LookUp`
  (params (AxisValue :type "Float (single-precision)"))
  ;[1 1 1] Turn
  (`self.AddControllerPitchInput` AxisValue))

(event `InputAxis|LadderUpDown`
  (params (AxisValue :type "Float (single-precision)"))
  (bind _animinstance (`self.AnimInstance`))
  (bind (_returnvalue_roll _returnvalue_pitch _returnvalue_yaw) (`KismetMathLibrary.BreakRotator` (`KismetMathLibrary.ComposeRotators` (`/Game/Firetruck/Meshes/SK_Ladder_Skeleton_AnimBlueprint.LadderUpDown` _animinstance) (`KismetMathLibrary.MakeRotator` 0.0 (* (`GameplayStatics.GetWorldDeltaSeconds`) AxisValue 8.0)))))
  ;[1 1 1] Ladder Movement
  (bind _output_get (set `/Game/Firetruck/Meshes/SK_Ladder_Skeleton_AnimBlueprint.LadderUpDown` (`KismetMathLibrary.MakeRotator` _returnvalue_roll (`KismetMathLibrary.FClamp` _returnvalue_pitch -1.75 55.0) _returnvalue_yaw) _animinstance))
  (`self.SetUpDown` _output_get))

(event `SetUpDown`
  (params (NewParam :type "Rotator Structure"))
  (bind _animinstance (`self.AnimInstance`))
  ;[1 1 1] Replicated
  (`/Engine/EditorBlueprintResources/StandardMacros.IsValid` _animinstance
    (:`Is Valid`
      (`/Engine/EditorBlueprintResources/ActorMacros.Switch Has Authority`
        (:`Remote`
          (set `/Game/Firetruck/Meshes/SK_Ladder_Skeleton_AnimBlueprint.LadderUpDown` NewParam _animinstance))))))

(event `InputAction|Lights`
  (params (Key :type "Key Structure"))
  ;[1 1 1] Flash Lights
  (:`Pressed`
    (`self.ToggleFlashLights` (`self.IsFlashLights`))
    (`self.TurnOnFlashLightsRPC` (not (`self.IsFlashLights`)))))

(event `InputAxis|LadderShift`
  (params (AxisValue :type "Float (single-precision)"))
  (bind _animinstance (`self.AnimInstance`))
  (bind (_returnvalue_x _returnvalue_y _returnvalue_z) (`KismetMathLibrary.BreakVector` (+ (`/Game/Firetruck/Meshes/SK_Ladder_Skeleton_AnimBlueprint.LadderShift` _animinstance) (`KismetMathLibrary.MakeVector` (* (`GameplayStatics.GetWorldDeltaSeconds`) AxisValue 70.0)))))
  ;[1 1 1] Ladder Movement
  (if (`self.EnableShift`)
    (bind _output_get (set `/Game/Firetruck/Meshes/SK_Ladder_Skeleton_AnimBlueprint.LadderShift` (`KismetMathLibrary.MakeVector` (`KismetMathLibrary.FClamp` _returnvalue_x 0.0 685.0) _returnvalue_y _returnvalue_z) _animinstance))
    (`self.SetShift` _output_get)))

(event `SetShift`
  (params (NewParam :type "Vector Structure"))
  (bind _animinstance (`self.AnimInstance`))
  ;[1 1 1] Replicated
  (`/Engine/EditorBlueprintResources/StandardMacros.IsValid` _animinstance
    (:`Is Valid`
      (`/Engine/EditorBlueprintResources/ActorMacros.Switch Has Authority`
        (:`Remote`
          (set `/Game/Firetruck/Meshes/SK_Ladder_Skeleton_AnimBlueprint.LadderShift` NewParam _animinstance))))))

(event `TurnOnFlashLightsRPC`
  (params (NewParam :type Boolean))
  ;[1 1 1] Flash Lights
  (`/Engine/EditorBlueprintResources/ActorMacros.Switch Has Authority`
    (:`Remote`
      (`self.ToggleFlashLights` NewParam))))

(fn `ToggleFlashLights`
  (params (NewParam :type Boolean))
  (bind _mesh (`self.Mesh`))
  (if NewParam
    (`/Engine/EditorBlueprintResources/StandardMacros.IsValid` (`self.FlashLights1`)
      (:`Is Valid`
        (`MaterialInstanceDynamic.SetScalarParameterValue` (`self.FlashLights1`) "LightPower" 0.0)
        (`MaterialInstanceDynamic.SetScalarParameterValue` (`self.FlashLights2`) "LightPower" 0.0)
        (set `self.IsFlashLights` false)))
    (else
      (`|ExecutionSequence`
        (:`then_0`
          (`/Engine/EditorBlueprintResources/StandardMacros.IsValid` (`self.FlashLights1`)
            (:`Is Not Valid`
              (bind _returnvalue (`PrimitiveComponent.CreateDynamicMaterialInstance` _mesh 7 "/Game/Firetruck/Materials/M_FiretruckSiren.M_FiretruckSiren" "None"))
              (set `self.FlashLights1` _returnvalue)
              (bind _returnvalue_2 (`PrimitiveComponent.CreateDynamicMaterialInstance` _mesh 8 "/Game/Firetruck/Materials/M_FiretruckSiren.M_FiretruckSiren" "None"))
              (set `self.FlashLights2` _returnvalue_2))))
        (:`then_1`
          (`MaterialInstanceDynamic.SetScalarParameterValue` (`self.FlashLights1`) "LightPower" 700.0)
          (`MaterialInstanceDynamic.SetScalarParameterValue` (`self.FlashLights2`) "LightPower" 700.0)
          (set `self.IsFlashLights` true))))))

(fn `UserConstructionScript`
  (bind _laddermesh (`self.LadderMesh`))
  (`SceneComponent.K2_SetWorldTransform` (`self.LadderCollision1`) (`SceneComponent.GetSocketTransform` _laddermesh "ladder_002" "RTS_World") false false)
  (`SceneComponent.K2_SetWorldTransform` (`self.LadderCollision2`) (`SceneComponent.GetSocketTransform` _laddermesh "ladder_001" "RTS_World") false false))