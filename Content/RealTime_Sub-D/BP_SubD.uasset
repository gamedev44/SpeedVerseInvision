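; Generated dynamic mesh actor that applies real-time Catmull-Clark subdivision to a copy of a target actor's mesh.
; Mesh rebuilds, plus an EditorTick timer set in construction, pass an activation toggle, then copy the target's root component mesh through Geometry Script.
; If the player-in-range flag is set, it subdivides by polygroup at the configured level.
; Failed copies or range checks print an error.
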(event `/Game/RealTime_Sub-D/BPI/BPI_Editor_Tick.EditorTick`
  (if (`self.Activate Realtime Sub-D`) :!label _label
    (bind _target_actor (`self.Target Actor`)
      (:`then`
        (bind _returnvalue (`BaseDynamicMeshComponent.GetDynamicMesh` (`self.DynamicMeshComponent`)))
        (bind (_localtoworld _returnvalue_2) (`GeometryScriptLibrary_SceneUtilityFunctions.CopyMeshFromComponent` (`Actor.RootComponent` _target_actor) _returnvalue (struct) false null)
          (:`Failure`
            (`KismetSystemLibrary.PrintString` "Player is Either Not in range for RTSD or Potentially SubD May Not Be found." true true (struct :`R` 1.0 :`G` 0.032916 :`A` 1.0) :!label _label_2))
          (:`Success`
            (if (`self.is player in range?`)
              (`GeometryScriptLibrary_OpenSubdivFunctions.ApplyPolygroupCatmullClarkSubD` _returnvalue_2 (`KismetMathLibrary.Conv_Int64ToInt` (`KismetMathLibrary.Conv_DoubleToInt64` (`self.Subdivisions`))) (struct) null)
              (else
                (goto _label_2))))))
      (:`else`))))

(event `self.OnRebuildGeneratedMesh`
  (params (TargetMesh :type "DynamicMesh Object Reference"))
  (goto _label))

(fn `UserConstructionScript`
  (`KismetSystemLibrary.K2_SetTimer` null "EditorTick" 0.25))