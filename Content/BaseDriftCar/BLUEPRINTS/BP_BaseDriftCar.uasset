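; Base Chaos vehicle pawn for a drivable drift car, with configurable meshes, materials, steering, traction control and per-axle friction.
; When player-controlled, Tick feeds inputs to the movement component and updates cameras, steering visuals, HUD and interior speedometers, engine audio and reverse lights.
; Tire skid effects derive from handbrake, lateral velocity and a ground trace, while speed limiting forces a gear or cuts torque.
; Input events handle lights, brake glow, camera switching and car flipping.
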(event `self.ReceiveBeginPlay`
  ;[0.3125 0 0 1 40] BEGIN PLAY EVENTS
  (if (`self.IsPlayerControlled`)
    (`self.Setup`)
    (bind _returnvalue (`|CreateWidget` "/Game/BaseDriftCar/HUD/HUD_SPEEDOMETER.HUD_SPEEDOMETER_C" (`GameplayStatics.GetPlayerController` 0) (`self.KmhOrMhp?`) (`self.SpeedometerColor1`) (`self.SpeedometerColor2`) (`self.SpeedometerGearColor`) (`self.SpeedometerSpeedColor`) (`self.ShowSpeedometer?`)))
    (bind _output_get (set `self.CAR SPEEDOMETER` _returnvalue))
    (`UserWidget.AddToViewport` _output_get 0)))

(event `self.ReceiveTick`
  (params (DeltaSeconds :type "Float (single-precision)"))
  (bind _tireskidactive_ (`self.TireSkidActive?`))
  (bind _mesh (`self.Mesh`))
  (bind _tireskidleft (`self.TireSkidLeft`))
  (bind _tirefloor_ (`self.TireFloor?`))
  (bind _tireskidright (`self.TireSkidRight`))
  (bind _returnvalue (* (`KismetMathLibrary.FClamp` (/ (- (`KismetMathLibrary.Abs` (`ChaosVehicleMovementComponent.GetForwardSpeed` (`self.VehicleMovementComponent`))) 55.0) 400.0) 0.0 0.7) (`KismetMathLibrary.Conv_BoolToDouble` (`self.HandBrake?`))))
  ;[0.06128 1 0 1 40] EVENT TICK
  (if (`self.IsPlayerControlled`)
    (`|ExecutionSequence`
      (:`then_0`
        (`self.Vehicle_Inputs`)
        (`self.Camera_Input`)
        (`self.InteriorCamera_Input`)
        (`self.SteeringWheelRotation` DeltaSeconds)
        (`self.Speedometer`)
        (`self.Gear&RPMSetup`)
        (`self.Car_Sound`)
        (`self.ReverseLights`)
        (`PrimitiveComponent.SetSimulatePhysics` (`self.Mesh`) true))
      (:`then_1`
        (`self.TireGroundCheck`)
        (if (`self.TireSkid?`)
          (bind _returnvalue_2 (`PrimitiveComponent.GetPhysicsLinearVelocity` _mesh "None"))
          (if _tireskidactive_
            (bind _y (.y (`KismetMathLibrary.LessLess_VectorRotator` _returnvalue_2 (`SceneComponent.K2_GetComponentRotation` _mesh))))
            (bind _returnvalue_3 (`KismetMathLibrary.FClamp` (+ _returnvalue (/ (`KismetMathLibrary.FClamp` (- (`KismetMathLibrary.Abs` (- _y 100.0)) 300.0) 0.0 1000.0) 500.0))))
            (bind _returnvalue_4 (and (> _returnvalue_3 0.0) _tirefloor_))
            (`ActorComponent.SetActive` _tireskidleft _returnvalue_4 false)
            (`ActorComponent.SetActive` (`self.TIRESKIDSOUND`) _returnvalue_4 false)
            (`ActorComponent.SetActive` _tireskidright _returnvalue_4 false)
            (`SceneComponent.SetVisibility` _tireskidleft _returnvalue_4 false)
            (`FXSystemComponent.SetFloatParameter` _tireskidleft "Opacity" _returnvalue_3)
            (`FXSystemComponent.SetFloatParameter` _tireskidright "Opacity" _returnvalue_3)
            (if _tireskidactive_
              (bind _returnvalue_5 (`KismetMathLibrary.FClamp` (+ _returnvalue (/ (`KismetMathLibrary.FClamp` (- (`KismetMathLibrary.Abs` (+ _y 100.0)) 300.0) 0.0 1000.0) 500.0))))
              (`ActorComponent.SetActive` _tireskidright (and _tirefloor_ (> _returnvalue_5 0.0)) false)
              (`SceneComponent.SetVisibility` _tireskidright _tireskidactive_ false)
              (`FXSystemComponent.SetFloatParameter` _tireskidright "Opacity" _returnvalue_5)))))
      (:`then_2`
        (`self.MaxSpeed`)))))

(event `Key|NumPadFour`
  (params (Key :type "Key Structure"))
  (bind _leftsidecamera (`self.LeftSideCamera`))
  (:`Pressed`
    (if (`ActorComponent.IsActive` (`self.MainCamera`))
      (`ActorComponent.SetActive` _leftsidecamera true false)
      (`ActorComponent.Deactivate` (`self.MainCamera`))
      (`ActorComponent.Deactivate` (`self.ExCam2`))
      (`ActorComponent.Deactivate` (`self.ExCam1`))
      (`ActorComponent.Deactivate` (`self.RearCam`))
      (`ActorComponent.Deactivate` (`self.RightSideCamera`))
      (`ActorComponent.Deactivate` (`self.RearSideCamera`))))
  (:`Released`
    (if (`ActorComponent.IsActive` (`self.LeftSideCamera`))
      (`ActorComponent.Deactivate` _leftsidecamera)
      (`ActorComponent.SetActive` (`self.MainCamera`) true true))))

(event `Key|NumPadSix`
  (params (Key :type "Key Structure"))
  (bind _rightsidecamera (`self.RightSideCamera`))
  (:`Pressed`
    (if (`ActorComponent.IsActive` (`self.MainCamera`))
      (`ActorComponent.SetActive` _rightsidecamera true false)
      (`ActorComponent.Deactivate` (`self.MainCamera`))
      (`ActorComponent.Deactivate` (`self.ExCam2`))
      (`ActorComponent.Deactivate` (`self.ExCam1`))
      (`ActorComponent.Deactivate` (`self.RearCam`))
      (`ActorComponent.Deactivate` (`self.LeftSideCamera`))
      (`ActorComponent.Deactivate` (`self.RearSideCamera`))))
  (:`Released`
    (if (`ActorComponent.IsActive` (`self.RightSideCamera`))
      (`ActorComponent.Deactivate` _rightsidecamera)
      (`ActorComponent.SetActive` (`self.MainCamera`) true true))))

(event `Key|NumPadTwo`
  (params (Key :type "Key Structure"))
  (bind _rearsidecamera (`self.RearSideCamera`))
  (:`Pressed`
    (if (`ActorComponent.IsActive` (`self.MainCamera`))
      (`ActorComponent.SetActive` _rearsidecamera true false)
      (`ActorComponent.Deactivate` (`self.MainCamera`))
      (`ActorComponent.Deactivate` (`self.ExCam2`))
      (`ActorComponent.Deactivate` (`self.ExCam1`))
      (`ActorComponent.Deactivate` (`self.RearCam`))
      (`ActorComponent.Deactivate` (`self.LeftSideCamera`))
      (`ActorComponent.Deactivate` (`self.RightSideCamera`))))
  (:`Released`
    (if (`ActorComponent.IsActive` (`self.RearSideCamera`))
      (`ActorComponent.Deactivate` _rearsidecamera)
      (`ActorComponent.SetActive` (`self.MainCamera`) true true))))

(event `Key|SpaceBar`
  (params (Key :type "Key Structure"))
  (:`Pressed`
    (if (> (`ChaosVehicleMovementComponent.GetForwardSpeed` (`self.VehicleMovementComponent`)) 1200.0)
      (bind (_direction _newtrack_0) (`Timeline|Timeline_0` :!label _label)
        (:`Update`
          (`MeshComponent.SetScalarParameterValueOnMaterials` (`self.WHEEL_FL`) "BrakeDiskEmmisive" _newtrack_0)
          (`MeshComponent.SetScalarParameterValueOnMaterials` (`self.WHEEL_FR`) "BrakeDiskEmmisive" _newtrack_0)
          (`MeshComponent.SetScalarParameterValueOnMaterials` (`self.Wheel_BR`) "BrakeDiskEmmisive" _newtrack_0)
          (`MeshComponent.SetScalarParameterValueOnMaterials` (`self.WHEEL_BL`) "BrakeDiskEmmisive" _newtrack_0)))))
  (:`Released`
    (goto _label :!via `Reverse`)))

(event `Setup`
  (bind _tractioncontrol (`self.TractionControl`))
  (bind _maxsteer (`self.MaxSteer`))
  (bind _aschaos_wheeled_vehicle_movement_component (cast `ChaosWheeledVehicleMovementComponent` (`self.VehicleMovementComponent`)))
  (`ChaosWheeledVehicleMovementComponent.SetWheelMaxSteerAngle` _aschaos_wheeled_vehicle_movement_component 0 _maxsteer)
  (`ChaosWheeledVehicleMovementComponent.SetWheelMaxSteerAngle` _aschaos_wheeled_vehicle_movement_component 1 _maxsteer)
  (`ChaosWheeledVehicleMovementComponent.SetTractionControlEnabled` _aschaos_wheeled_vehicle_movement_component 0 _tractioncontrol)
  (`ChaosWheeledVehicleMovementComponent.SetTractionControlEnabled` _aschaos_wheeled_vehicle_movement_component 1 _tractioncontrol)
  (`ChaosWheeledVehicleMovementComponent.SetTractionControlEnabled` _aschaos_wheeled_vehicle_movement_component 2 _tractioncontrol)
  (`ChaosWheeledVehicleMovementComponent.SetTractionControlEnabled` _aschaos_wheeled_vehicle_movement_component 3 _tractioncontrol)
  (set `self.FrontWheelsLocation` (`self.FrontWheelsLocation`))
  (set `self.BackWheelsLocation` (`self.BackWheelsLocation`))
  (`ChaosWheeledVehicleMovementComponent.SetWheelFrictionMultiplier` _aschaos_wheeled_vehicle_movement_component 2 (`self.BackWheelsSliping`))
  (`ChaosWheeledVehicleMovementComponent.SetWheelFrictionMultiplier` _aschaos_wheeled_vehicle_movement_component 3 (`self.BackWheelsSliping`))
  (`ChaosWheeledVehicleMovementComponent.SetWheelFrictionMultiplier` _aschaos_wheeled_vehicle_movement_component 0 (`self.FrontWheelsSliping`))
  (`ChaosWheeledVehicleMovementComponent.SetWheelFrictionMultiplier` _aschaos_wheeled_vehicle_movement_component 1 (`self.FrontWheelsSliping`))
  (`ChaosWheeledVehicleMovementComponent.SetMaxEngineTorque` _aschaos_wheeled_vehicle_movement_component (`self.EngineTorque`))
  (`CameraComponent.SetFieldOfView` (`self.MainCamera`) (`self.CameraFieldOfView`)))

(event `InputAction|SwitchCamera`
  (params (Key :type "Key Structure"))
  (bind _car_speedometer (`self.CAR SPEEDOMETER`))
  (bind _maincamera (`self.MainCamera`))
  (bind _interiorcamera (`self.InteriorCamera`))
  (:`Pressed`
    (`/Engine/EditorBlueprintResources/StandardMacros.FlipFlop`
      (:`A`
        (`ActorComponent.Activate` _interiorcamera false)
        (`ActorComponent.Deactivate` _maincamera)
        (`Widget.SetVisibility` _car_speedometer "Hidden"))
      (:`B`
        (`ActorComponent.Activate` _maincamera false)
        (`ActorComponent.Deactivate` _interiorcamera)
        (`Widget.SetVisibility` _car_speedometer "Visible")))))

(event `Key|MouseScrollDown`
  (params (Key :type "Key Structure"))
  (bind _mainspringarm (`self.MainSpringArm`))
  (:`Pressed`
    (set `SpringArmComponent.TargetArmLength` (+ (`KismetMathLibrary.FClamp` (`SpringArmComponent.TargetArmLength` _mainspringarm) 400.0 2000.0) 20.0) _mainspringarm)))

(event `Key|MouseScrollUp`
  (params (Key :type "Key Structure"))
  (bind _mainspringarm (`self.MainSpringArm`))
  (:`Pressed`
    (set `SpringArmComponent.TargetArmLength` (- (`KismetMathLibrary.FClamp` (`SpringArmComponent.TargetArmLength` _mainspringarm) 400.0 2000.0) 20.0) _mainspringarm)))

(event `InputAction|Lights`
  (params (Key :type "Key Structure"))
  (:`Pressed`
    (`/Engine/EditorBlueprintResources/StandardMacros.FlipFlop`
      (:`A`
        (`SceneComponent.SetVisibility` (`self.FLightRight`) true false)
        (`SceneComponent.SetVisibility` (`self.FLightLeft`) true false)
        (`SceneComponent.SetVisibility` (`self.BACKLIGHTRIGHT`) true false)
        (`SceneComponent.SetVisibility` (`self.BACKLIGHTLEFT`) true false)
        (`SceneComponent.SetVisibility` (`self.BACK LEFT OPENABLE LIGHT`) true false)
        (`SceneComponent.SetVisibility` (`self.FrontLeftLightGlow`) true false)
        (`SceneComponent.SetVisibility` (`self.FrontRightLightGlow`) true false)
        (`SceneComponent.SetVisibility` (`self.BACK RIGHT OPENABLE LIGHT`) true false)
        (`SceneComponent.SetVisibility` (`self.BACK DECOR LIGHT`) true false))
      (:`B`
        (`SceneComponent.SetVisibility` (`self.FLightLeft`) false false)
        (`SceneComponent.SetVisibility` (`self.FLightRight`) false false)
        (`SceneComponent.SetVisibility` (`self.BACKLIGHTRIGHT`) false false)
        (`SceneComponent.SetVisibility` (`self.BACKLIGHTLEFT`) false false)
        (`SceneComponent.SetVisibility` (`self.BACK LEFT OPENABLE LIGHT`) false false)
        (`SceneComponent.SetVisibility` (`self.FrontLeftLightGlow`) false false)
        (`SceneComponent.SetVisibility` (`self.FrontRightLightGlow`) false false)
        (`SceneComponent.SetVisibility` (`self.BACK RIGHT OPENABLE LIGHT`) false false)
        (`SceneComponent.SetVisibility` (`self.BACK DECOR LIGHT`) false false)))))

(event `Key|SpaceBar`
  (params (Key :type "Key Structure"))
  (:`Pressed`
    (`self.StopLights` :!label _label_2))
  (:`Released`
    (goto _label_2 :!via `InputPin`)))

(event `Key|X`
  (params (Key :type "Key Structure"))
  ;[0 0 0 1 40] TURN KMH OR MPH
  (:`Pressed`
    (`/Engine/EditorBlueprintResources/StandardMacros.FlipFlop`
      (:`A`
        (set `self.KmhOrMhp?` false))
      (:`B`
        (set `self.KmhOrMhp?` true)))))

(event `Key|R`
  (params (Key :type "Key Structure"))
  ;[0 0 0 1 40] FLIP CAR
  (:`Pressed`
    (`self.FlipCar`)))

(event `InputAction|Handbrake`
  (params (Key :type "Key Structure"))
  (bind _vehiclemovementcomponent (`self.VehicleMovementComponent`))
  ;[0 0 0] HANDBRAKE
  (:`Pressed`
    (`ChaosVehicleMovementComponent.SetHandbrakeInput` _vehiclemovementcomponent true))
  (:`Released`
    (`ChaosVehicleMovementComponent.SetHandbrakeInput` _vehiclemovementcomponent false)))

(fn `Camera_Input`
  (bind (_returnvalue_roll _returnvalue_pitch _returnvalue_yaw) (`KismetMathLibrary.BreakRotator` (`SceneComponent.K2_GetComponentRotation` (`self.MainCameraRef`))))
  (if (`self.CameraRotationInvert?`)
    (`SceneComponent.K2_AddRelativeRotation` (`self.MainSpringArm`) (`KismetMathLibrary.MakeRotator` 0.0 (* (`self.GetInputAxisValue`) -1.0) (`self.GetInputAxisValue`)) false false)
    (else
      (`SceneComponent.K2_AddRelativeRotation` (`self.MainSpringArm`) (`KismetMathLibrary.MakeRotator` 0.0 (`self.GetInputAxisValue`) (`self.GetInputAxisValue`)) false false)
      (if (`self.CameraAutoCentering?`)
        (if (> (* (`ChaosVehicleMovementComponent.GetForwardSpeed` (`self.VehicleMovementComponent`)) 0.036) (`self.CameraAutoCenterStartSpeed`))
          (`SceneComponent.K2_SetWorldRotation` (`self.MainSpringArm`) (`KismetMathLibrary.MakeRotator` _returnvalue_roll _returnvalue_pitch _returnvalue_yaw) false false)
          (`SceneComponent.K2_SetWorldRotation` (`self.InteriorSpringArm`) (`KismetMathLibrary.MakeRotator` _returnvalue_roll _returnvalue_pitch _returnvalue_yaw) false false))))))

(fn `Car_Sound`
  (bind _enginesound (`self.EngineSound`))
  (if (`self.EngineSound?`)
    (`AudioComponent.SetFloatParameter` _enginesound "RPM" (* (`ChaosVehicleMovementComponent.GetForwardSpeed` (`self.VehicleMovementComponent`)) (`self.EngineSoundRpmMultiplier`)))
    (`AudioComponent.SetVolumeMultiplier` _enginesound (`self.EngineSoundVolume`))
    (`AudioComponent.SetPitchMultiplier` _enginesound (`self.EngineSoundPitch`))))

(fn `FlipCar`
  (bind (_returnvalue_x _returnvalue_y _returnvalue_z) (`KismetMathLibrary.BreakVector` (`self.K2_GetActorLocation`)))
  (bind (_returnvalue_roll _returnvalue_pitch _returnvalue_yaw) (`KismetMathLibrary.BreakRotator` (`self.K2_GetActorRotation`)))
  (`self.K2_SetActorTransform` (`KismetMathLibrary.MakeTransform` (`KismetMathLibrary.MakeVector` _returnvalue_x _returnvalue_y (+ _returnvalue_z 200.0)) (`KismetMathLibrary.MakeRotator` 0.0 0.0 _returnvalue_yaw)) false true))

(fn `Gear&RPMSetup`
  (bind _vehiclemovementcomponent (`self.VehicleMovementComponent`))
  (set `self.VehicleSpeed` (`ChaosVehicleMovementComponent.GetForwardSpeed` _vehiclemovementcomponent))
  (set `self.CurrentGear` (`ChaosVehicleMovementComponent.GetCurrentGear` _vehiclemovementcomponent))
  (set `self.VehicleRPM` (`KismetMathLibrary.FInterpTo` (`self.VehicleRPM`) (`KismetMathLibrary.FClamp` (`ChaosWheeledVehicleMovementComponent.GetEngineRotationSpeed` (cast `ChaosWheeledVehicleMovementComponent` _vehiclemovementcomponent :!pure true)) 0.0 8000.0) (`GameplayStatics.GetTimeSeconds`))))

(fn `InteriorCamera_Input`
  (`SceneComponent.K2_AddRelativeRotation` (`self.InteriorSpringArm`) (`KismetMathLibrary.MakeRotator` 0.0 (`self.GetInputAxisValue`) (`self.GetInputAxisValue`)) false false))

(fn `MaxSpeed`
  (if (`self.SpeedOrGearBasedLimit`)
    ;[1 1 1] GEAR BASED SPEED LIMIT
    (if (> (* (`ChaosVehicleMovementComponent.GetForwardSpeed` (`self.VehicleMovementComponent`)) 0.036) (`self.SpeedLimitKM`))
      (`ChaosVehicleMovementComponent.SetTargetGear` (`self.VehicleMovementComponent`) 2 true))
    (else
      ;[1 1 1] SPEED BASED SPEED LIMIT
      (if (> (* (`ChaosVehicleMovementComponent.GetForwardSpeed` (`self.VehicleMovementComponent`)) 0.036) (`self.SpeedLimitKM`))
        (bind _aschaos_wheeled_vehicle_movement_component (cast `ChaosWheeledVehicleMovementComponent` (`self.VehicleMovementComponent`)))
        (`ChaosWheeledVehicleMovementComponent.SetMaxEngineTorque` _aschaos_wheeled_vehicle_movement_component 1000.0)
        (else
          (bind _aschaos_wheeled_vehicle_movement_component_2 (cast `ChaosWheeledVehicleMovementComponent` (`self.VehicleMovementComponent`)))
          (`ChaosWheeledVehicleMovementComponent.SetMaxEngineTorque` _aschaos_wheeled_vehicle_movement_component_2 50000.0))))))

(fn `ReverseLights`
  (bind _reverselightleft (`self.ReverseLightLeft`))
  (if (< (`ChaosVehicleMovementComponent.GetForwardSpeed` (`self.VehicleMovementComponent`)) -40.0)
    (`SceneComponent.SetVisibility` _reverselightleft true false)
    (`SceneComponent.SetVisibility` (`self.ReverseLightRight`) true false)
    (`SceneComponent.SetVisibility` (`self.LEFT REAR LIGHT`) true false)
    (`SceneComponent.SetVisibility` (`self.RIGHT REAR LIGHT`) true false)
    (else
      (`SceneComponent.SetVisibility` _reverselightleft false false)
      (`SceneComponent.SetVisibility` (`self.ReverseLightRight`) false false)
      (`SceneComponent.SetVisibility` (`self.LEFT REAR LIGHT`) false false)
      (`SceneComponent.SetVisibility` (`self.RIGHT REAR LIGHT`) false false))))

(fn `Speedometer`
  (bind _vehiclerpm (`self.VehicleRPM`))
  (bind _car_speedometer (`self.CAR SPEEDOMETER`))
  (bind _returnvalue (`ChaosVehicleMovementComponent.GetForwardSpeed` (`self.VehicleMovementComponent`)))
  (bind _returnvalue_2 (`KismetTextLibrary.Conv_StringToText` (`self.GearDispText`)))
  (bind _returnvalue_3 (`KismetMathLibrary.FFloor` (`KismetMathLibrary.Abs` (* _returnvalue 0.036))))
  (`|ExecutionSequence`
    (:`then_0`
      (if (`self.KmhOrMhp?`)
        (set `/Game/BaseDriftCar/HUD/HUD_SPEEDOMETER.SpeedHUD` _returnvalue_3 _car_speedometer)
        (else
          (bind _output_get (set `/Game/BaseDriftCar/HUD/HUD_SPEEDOMETER.SpeedHUD` (`KismetMathLibrary.FFloor` (`KismetMathLibrary.Abs` (* _returnvalue 0.022))) (`self.CAR SPEEDOMETER`)))
          (bind _ashud_speedometer_int (cast `/Game/BaseDriftCar/HUD/HUD_SPEEDOMETER_INT` (`WidgetComponent.GetUserWidgetObject` (`self.SpeedometerRPM_Interior`))))
          (set `/Game/BaseDriftCar/HUD/HUD_SPEEDOMETER_INT.SpeedHUD` _output_get _ashud_speedometer_int)))
      (set `/Game/BaseDriftCar/HUD/HUD_SPEEDOMETER.RPM` (`self.VehicleRPM`) _car_speedometer)
      (set `/Game/BaseDriftCar/HUD/HUD_SPEEDOMETER.GearText` _returnvalue_2 _car_speedometer)
      (set `/Game/BaseDriftCar/HUD/HUD_SPEEDOMETER.KmhOrMph` (`self.KmhOrMhp?`) _car_speedometer)
      (set `/Game/BaseDriftCar/HUD/HUD_SPEEDOMETER.SpeedometerColor1` (`self.SpeedometerColor1`) _car_speedometer)
      (set `/Game/BaseDriftCar/HUD/HUD_SPEEDOMETER.SpeedometerColor2` (`self.SpeedometerColor2`) _car_speedometer)
      (set `/Game/BaseDriftCar/HUD/HUD_SPEEDOMETER.SpeedometerGearColor` (`self.SpeedometerGearColor`) _car_speedometer)
      (set `/Game/BaseDriftCar/HUD/HUD_SPEEDOMETER.SpeedometerSpeedColor` (`self.SpeedometerSpeedColor`) _car_speedometer)
      (bind _ashud_speedometer_int_2 (cast `/Game/BaseDriftCar/HUD/HUD_SPEEDOMETER_INT` (`WidgetComponent.GetUserWidgetObject` (`self.SpeedometerRPM_Interior`))))
      (set `/Game/BaseDriftCar/HUD/HUD_SPEEDOMETER_INT.RPM` _vehiclerpm _ashud_speedometer_int_2)
      (set `/Game/BaseDriftCar/HUD/HUD_SPEEDOMETER_INT.VehicleSpeed` (`self.VehicleSpeed`) _ashud_speedometer_int_2)
      (set `/Game/BaseDriftCar/HUD/HUD_SPEEDOMETER_INT.VehicleRpm` _vehiclerpm _ashud_speedometer_int_2)
      (set `/Game/BaseDriftCar/HUD/HUD_SPEEDOMETER_INT.KmhorMph` (`self.KmhOrMhp?`) _ashud_speedometer_int_2)
      (set `/Game/BaseDriftCar/HUD/HUD_SPEEDOMETER_INT.GearText` _returnvalue_2 _ashud_speedometer_int_2)
      (if (`self.KmhOrMhp?`)
        (set `/Game/BaseDriftCar/HUD/HUD_SPEEDOMETER_INT.SpeedHUD` _returnvalue_3 _ashud_speedometer_int_2)))
    (:`then_1`
      (bind _output_get_2 (set `self.CurrentGear` (`self.CurrentGear`)))
      (if (< _output_get_2 0)
        (set `self.GearDispText` "R")
        (elif (> (`self.CurrentGear`) 0)
          (set `self.GearDispText` (`KismetStringLibrary.Conv_IntToString` (`self.CurrentGear`)))
          (else
            (set `self.GearDispText` "N")))))))

(fn `SteeringWheelRotation`
  (params (DeltaSec :type "Float (double-precision)"))
  (bind _steeringwheel_mesh (`self.SteeringWheel Mesh`))
  (bind _aschaos_wheeled_vehicle_movement_component (cast `ChaosWheeledVehicleMovementComponent` (`self.VehicleMovementComponent`)))
  (`|ExecutionSequence`
    (:`then_0`
      (bind _wheels (`ChaosWheeledVehicleMovementComponent.Wheels` _aschaos_wheeled_vehicle_movement_component))
      (bind _returnvalue (`ChaosVehicleWheel.GetSteerAngle` (`|GetArrayItem` _wheels)))
      (bind _returnvalue_2 (`ChaosVehicleWheel.GetSteerAngle` (`|GetArrayItem` _wheels 1)))
      (bind _returnvalue_3 (`KismetMathLibrary.SelectFloat` _returnvalue _returnvalue_2 (>= (`KismetMathLibrary.Abs` _returnvalue) (`KismetMathLibrary.Abs` _returnvalue_2))))
      (`SceneComponent.K2_SetRelativeRotation` _steeringwheel_mesh (`KismetMathLibrary.MakeRotator` _returnvalue_3 -30.0) false false)
      (`SceneComponent.K2_SetRelativeRotation` (`self.CALIPER_FR`) (`KismetMathLibrary.MakeRotator` 0.0 0.0 _returnvalue_3) false false))
    (:`then_1`
      (`SceneComponent.K2_SetRelativeRotation` _steeringwheel_mesh (`KismetMathLibrary.MakeRotator` _returnvalue_3 -30.0) false false)
      (`SceneComponent.K2_SetRelativeRotation` (`self.CALIPER_FL`) (`KismetMathLibrary.MakeRotator` 0.0 0.0 _returnvalue_3) false false))))

(fn `TireGroundCheck`
  (bind _returnvalue_location (`KismetMathLibrary.BreakTransform` (`SceneComponent.K2_GetComponentToWorld` (`self.SkidmarkFloorCheck`))))
  (bind (_outhit _returnvalue) (`KismetSystemLibrary.LineTraceSingle` (+ _returnvalue_location (0.0 0.0 0.0)) (- _returnvalue_location (0.0 0.0 30.0)) "TraceTypeQuery1"))
  (set `self.TireFloor?` _returnvalue))

(fn `UserConstructionScript`
  (bind _wheelmeshes (`self.WheelMeshes`))
  (`StaticMeshComponent.SetStaticMesh` (`self.BODY ( PLACE YOUR MESH )`) (`self.Body Mesh`))
  (`StaticMeshComponent.SetStaticMesh` (`self.WHEEL_FR`) _wheelmeshes)
  (`StaticMeshComponent.SetStaticMesh` (`self.WHEEL_FL`) _wheelmeshes)
  (`StaticMeshComponent.SetStaticMesh` (`self.Wheel_BR`) _wheelmeshes)
  (`StaticMeshComponent.SetStaticMesh` (`self.WHEEL_BL`) _wheelmeshes)
  (`StaticMeshComponent.SetStaticMesh` (`self.SPOILER`) (`self.SpoilerMesh`))
  (`StaticMeshComponent.SetStaticMesh` (`self.SteeringWheel Mesh`) (`self.Steering Wheel Mesh`))
  (`PrimitiveComponent.SetMaterial` (`self.BODY ( PLACE YOUR MESH )`) (`self.BodyMaterialIndex`) (`self.BodyMaterial`))
  (`PrimitiveComponent.SetMaterial` (`self.WHEEL_FL`) (`self.WheelMaterialIndex`) (`self.WheelMaterial`))
  (`PrimitiveComponent.SetMaterial` (`self.WHEEL_FR`) (`self.WheelMaterialIndex`) (`self.WheelMaterial`))
  (`PrimitiveComponent.SetMaterial` (`self.Wheel_BR`) (`self.WheelMaterialIndex`) (`self.WheelMaterial`))
  (`PrimitiveComponent.SetMaterial` (`self.WHEEL_BL`) (`self.WheelMaterialIndex`) (`self.WheelMaterial`))
  (`PrimitiveComponent.SetMaterial` (`self.SteeringWheel Mesh`) 0 (`self.Steering Wheel Material`)))

(fn `Vehicle_Inputs`
  (bind _vehiclemovementcomponent (`self.VehicleMovementComponent`))
  ;[0 0 0 1 30] VEHICLE INPUTS
  (`ChaosVehicleMovementComponent.SetBrakeInput` _vehiclemovementcomponent (`self.GetInputAxisValue`))
  (`ChaosVehicleMovementComponent.SetSteeringInput` _vehiclemovementcomponent (`self.GetInputAxisValue`))
  (`ChaosVehicleMovementComponent.SetThrottleInput` _vehiclemovementcomponent (`self.GetInputAxisValue`))
  (if (`self.Z-Force?`)
    (`PrimitiveComponent.AddForce` (`self.Mesh`) (`KismetMathLibrary.MakeVector` 0.0 0.0 (* (`self.Z-Force`) -1.0)) "DYNO_ROOT" true)))