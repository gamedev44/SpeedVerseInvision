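; Actor that records the player sports car's path as a spline for police AI to follow and spawns chasing police cars on it.
; Delay loops sample the car's position, keeping points at least 100 units apart and trimming the oldest at a maximum length.
; Once full, it spawns BP_AI_Police at a fixed spline point while under the chaser cap and wanted, with intervals set by the polled wanted level.
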(event `self.ReceiveBeginPlay`
  (bind _returnvalue (`self.K2_GetActorLocation`))
  (bind _spline (`self.Spline`))
  (bind _wantedlevel (`self.WantedLevel`))
  (bind _returnvalue_2 (`SplineComponent.GetRotationAtSplinePoint` _spline 65 "World"))
  (bind (_returnvalue_x _returnvalue_y _returnvalue_z) (`KismetMathLibrary.BreakVector` (`SplineComponent.GetLocationAtSplinePoint` _spline 65 "World")))
  (bind _returnvalue_location (`KismetMathLibrary.BreakTransform` (`SceneComponent.K2_GetComponentToWorld` (`/Game/PoliceAI/Blueprints/BP_Pawn_SportsCar.DrawTraceLocation` (`self.As BP Sports Car Pawn`)))))
  (bind _returnvalue_3 (- _returnvalue_z 40.0))
  ;[1 1 1] Get Player Wanted Level
  (bind _asbp_pawn_sports_car (cast `/Game/PoliceAI/Blueprints/BP_Pawn_SportsCar` (`GameplayStatics.GetPlayerPawn` 0) :!label _label))
  (set `self.WantedLevel` (`|GetEnumeratorNameAsString` (`/Game/PoliceAI/Blueprints/BP_Pawn_SportsCar.WantedLevel` _asbp_pawn_sports_car)))
  (`|ExecutionSequence`
    (:`then_0`
      (`KismetSystemLibrary.Delay` 1.0)
      (goto _label))
    (:`then_1`
      (`/Engine/EditorBlueprintResources/StandardMacros.DoOnce` false
        (:`Completed`
          (set `self.As BP Sports Car Pawn` _asbp_pawn_sports_car)
          ;[1 1 1] Draw Chased Vehicle Trace for Police AI to Follow
          (`|ExecutionSequence`
            (:`then_0`
              (`SplineComponent.SetLocationAtSplinePoint` (`self.Spline`) 0 _returnvalue "World" true)
              (set `self.SplinePointComparisonValue1` _returnvalue)
              (`SplineComponent.AddSplinePointAtIndex` (`self.Spline`) _returnvalue_location (`self.Point Index`) "World" true :!label _label_2)
              (set `self.SplinePointComparisonValue2` _returnvalue_location)
              (if (>= (`KismetMathLibrary.VSize` (- (`self.SplinePointComparisonValue1`) (`self.SplinePointComparisonValue2`))) 100.0)
                (`/Engine/EditorBlueprintResources/StandardMacros.IncrementInt` (`self.Point Index`)
                  (:`  `
                    (set `self.SplinePointComparisonValue1` (`self.SplinePointComparisonValue2`))))
                (else
                  (`SplineComponent.RemoveSplinePoint` (`self.Spline`) (`self.Point Index`) true)))
              (if (>= (`SplineComponent.GetSplineLength` (`self.Spline`)) (`self.MaxTraceLength`))
                (set `self.Point Index` (- (`SplineComponent.GetNumberOfSplinePoints` (`self.Spline`)) 1))
                (`SplineComponent.RemoveSplinePoint` (`self.Spline`) 0 true)
                (`|ExecutionSequence`
                  (:`then_0`
                    (`KismetSystemLibrary.Delay` 0.05 :!label _label_3)
                    (goto _label_2))
                  (:`then_1`
                    ;[1 1 1] Spawn Police AI
                    (if (< (`/Game/PoliceAI/Blueprints/BP_Pawn_SportsCar.NumberOfChasingPoliceCars` _asbp_pawn_sports_car) (`self.MaxPoliceAI SpawnNumber`))
                      (`KismetSystemLibrary.Delay` (`self.PoliceAI SpawnRateInSeconds`))
                      (bind _asbp_pawn_sports_car_2 (cast `/Game/PoliceAI/Blueprints/BP_Pawn_SportsCar` (`GameplayStatics.GetPlayerPawn` 0)))
                      (if (`KismetStringLibrary.StartsWith` (`|GetEnumeratorNameAsString` (`/Game/PoliceAI/Blueprints/BP_Pawn_SportsCar.WantedLevel` _asbp_pawn_sports_car_2)) "No")
                        _
                        (elif (`KismetStringLibrary.Contains` (`self.WantedLevel`) "5")
                          ;[1 0 0.02496] Level 5 Vehicle Spawn Class
                          (`|SpawnActorFromClass` "/Game/PoliceAI/AI/BP_AI_Police.BP_AI_Police_C" (`KismetMathLibrary.MakeTransform` (`KismetMathLibrary.MakeVector` _returnvalue_x _returnvalue_y _returnvalue_3) _returnvalue_2) "DontSpawnIfColliding" "MultiplyWithRoot" null true null)
                          (else
                            ;[1 1 1] Level 1-4 Vehicle Spawn Class
                            (`|SpawnActorFromClass` "/Game/PoliceAI/AI/BP_AI_Police.BP_AI_Police_C" (`KismetMathLibrary.MakeTransform` (`KismetMathLibrary.MakeVector` _returnvalue_x _returnvalue_y _returnvalue_3) _returnvalue_2) "DontSpawnIfColliding" "MultiplyWithRoot" null true null)))))))
                (else
                  (goto _label_3))))
            (:`then_1`
              (`KismetSystemLibrary.K2_SetTimer` null "SpawnRateCalculation" 2.0 true))))))
    (:`then_2`
      ;[1 1 1] Calculate Police AI Spawn Rate in Seconds
      (if (`KismetStringLibrary.EndsWith` _wantedlevel "1") :!label _label_4
        (set `self.PoliceAI SpawnRateInSeconds` (`KismetMathLibrary.Conv_IntToDouble` (`self.Level1 PoliceSpawnInterval (sec)`)))
        (elif (`KismetStringLibrary.EndsWith` _wantedlevel "2")
          (set `self.PoliceAI SpawnRateInSeconds` (`KismetMathLibrary.Conv_IntToDouble` (`self.Level2 PoliceSpawnInterval (sec)`)))
          (elif (`KismetStringLibrary.EndsWith` _wantedlevel "3")
            (set `self.PoliceAI SpawnRateInSeconds` (`KismetMathLibrary.Conv_IntToDouble` (`self.Level3 PoliceSpawnInterval (sec)`)))
            (elif (`KismetStringLibrary.EndsWith` _wantedlevel "4")
              (set `self.PoliceAI SpawnRateInSeconds` (`KismetMathLibrary.Conv_IntToDouble` (`self.Level4 PoliceSpawnInterval (sec)`)))
              (elif (`KismetStringLibrary.EndsWith` _wantedlevel "5")
                (set `self.PoliceAI SpawnRateInSeconds` (`KismetMathLibrary.Conv_IntToDouble` (`self.Level5 PoliceSpawnInterval (sec)`)))
                (else
                  (`KismetSystemLibrary.Delay` 2.0)
                  (goto _label_4))))))))))

(event `self.ReceiveTick`
  (params (DeltaSeconds :type "Float (single-precision)")))

(fn `UserConstructionScript`)