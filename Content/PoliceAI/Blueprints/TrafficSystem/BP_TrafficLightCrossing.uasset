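; Traffic light crossing actor that alternates two opposing pairs of signals (A and B) between green, yellow and red.
; BeginPlay spawns stop zones for side A, loops six timed light phases endlessly and enables physics on the light meshes.
; Each phase swaps material slots to new emissive dynamic instances or a default material.
; Phases 3 and 6 move the BP_TrafficLightStopZone actors between sides by destroying and respawning them at marker components.
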(event `self.ReceiveActorBeginOverlap`
  (params (OtherActor :type "Actor Object Reference")))

(event `self.ReceiveTick`
  (params (DeltaSeconds :type "Float (single-precision)")))

(event `self.ReceiveBeginPlay`
  (`|ExecutionSequence`
    (:`then_0`
      ;[1 1 1] Call Light Sequence Functions in Specific Order
      (`self.PreContruct`)
      (`self.LightSequence1` :!label _label)
      (`KismetSystemLibrary.Delay` (`self.LightSequenceIntervalInSeconds`))
      (`self.LightSequence2`)
      (`KismetSystemLibrary.Delay` (`self.YellowLightSequenceInterval`))
      (`self.LightSequence3`)
      (`KismetSystemLibrary.Delay` (`self.YellowLightSequenceInterval`))
      (`self.LightSequence4`)
      (`KismetSystemLibrary.Delay` (`self.LightSequenceIntervalInSeconds`))
      (`self.LightSequence5`)
      (`KismetSystemLibrary.Delay` (`self.YellowLightSequenceInterval`))
      (`self.LightSequence6`)
      (`KismetSystemLibrary.Delay` (`self.YellowLightSequenceInterval`))
      (goto _label))
    (:`then_1`
      ;[1 1 1] Activate Traffic Light Physics Simulation
      (`PrimitiveComponent.SetSimulatePhysics` (`self.TrafficLightGreenStartB1`) true)
      (`PrimitiveComponent.SetSimulatePhysics` (`self.TrafficLightGreenStartB2`) true)
      (`PrimitiveComponent.SetSimulatePhysics` (`self.TrafficLightRedStartA1`) true)
      (`PrimitiveComponent.SetSimulatePhysics` (`self.TrafficLightRedStartA2`) true))))

(fn `LightSequence1`
  (bind _trafficlightgreenstartb1 (`self.TrafficLightGreenStartB1`))
  (bind _trafficlightredstarta2 (`self.TrafficLightRedStartA2`))
  ;[1 1 1] Light Sequence 1
  (`|ExecutionSequence`
    (:`then_0`
      (bind _returnvalue (`KismetMaterialLibrary.CreateDynamicMaterialInstance` "/Game/PoliceAI/Materials/TrafficLightMaterials/MaterialInstances/MI_GreenTrafficLight.MI_GreenTrafficLight" "None"))
      (`PrimitiveComponent.SetMaterial` _trafficlightgreenstartb1 (`self.GreenTrafficLight`) _returnvalue)
      (`PrimitiveComponent.SetMaterial` (`self.TrafficLightGreenStartB2`) (`self.GreenTrafficLight`) _returnvalue)
      (`PrimitiveComponent.SetMaterial` _trafficlightgreenstartb1 (`self.YellowTrafficLight`) "/Game/PoliceAI/Materials/TrafficLightMaterials/M_DefaultMaterial.M_DefaultMaterial")
      (`PrimitiveComponent.SetMaterial` (`self.TrafficLightGreenStartB2`) (`self.YellowTrafficLight`) "/Game/PoliceAI/Materials/TrafficLightMaterials/M_DefaultMaterial.M_DefaultMaterial")
      (`PrimitiveComponent.SetMaterial` (`self.TrafficLightGreenStartB2`) (`self.RedTrafficLight`) "/Game/PoliceAI/Materials/TrafficLightMaterials/M_DefaultMaterial.M_DefaultMaterial")
      (`PrimitiveComponent.SetMaterial` _trafficlightgreenstartb1 (`self.RedTrafficLight`) "/Game/PoliceAI/Materials/TrafficLightMaterials/M_DefaultMaterial.M_DefaultMaterial")
      (`MaterialInstanceDynamic.SetScalarParameterValue` _returnvalue "Emissive" 15.0))
    (:`then_1`
      (bind _returnvalue_2 (`KismetMaterialLibrary.CreateDynamicMaterialInstance` "/Game/PoliceAI/Materials/TrafficLightMaterials/MaterialInstances/MI_RedTrafficLight.MI_RedTrafficLight" "None"))
      (`PrimitiveComponent.SetMaterial` _trafficlightredstarta2 (`self.RedTrafficLight`) _returnvalue_2)
      (`PrimitiveComponent.SetMaterial` (`self.TrafficLightRedStartA1`) (`self.RedTrafficLight`) _returnvalue_2)
      (`PrimitiveComponent.SetMaterial` _trafficlightredstarta2 (`self.YellowTrafficLight`) "/Game/PoliceAI/Materials/TrafficLightMaterials/M_DefaultMaterial.M_DefaultMaterial")
      (`PrimitiveComponent.SetMaterial` (`self.TrafficLightRedStartA1`) (`self.YellowTrafficLight`) "/Game/PoliceAI/Materials/TrafficLightMaterials/M_DefaultMaterial.M_DefaultMaterial")
      (`PrimitiveComponent.SetMaterial` _trafficlightredstarta2 (`self.GreenTrafficLight`) "/Game/PoliceAI/Materials/TrafficLightMaterials/M_DefaultMaterial.M_DefaultMaterial")
      (`PrimitiveComponent.SetMaterial` (`self.TrafficLightRedStartA1`) (`self.GreenTrafficLight`) "/Game/PoliceAI/Materials/TrafficLightMaterials/M_DefaultMaterial.M_DefaultMaterial")
      (`MaterialInstanceDynamic.SetScalarParameterValue` _returnvalue_2 "Emissive" 15.0))))

(fn `LightSequence2`
  (bind _trafficlightgreenstartb1 (`self.TrafficLightGreenStartB1`))
  (bind _trafficlightredstarta2 (`self.TrafficLightRedStartA2`))
  ;[1 1 1] Light Sequence 2
  (`|ExecutionSequence`
    (:`then_0`
      (bind _returnvalue (`KismetMaterialLibrary.CreateDynamicMaterialInstance` "/Game/PoliceAI/Materials/TrafficLightMaterials/MaterialInstances/MI_YellowTrafficLight.MI_YellowTrafficLight" "None"))
      (`PrimitiveComponent.SetMaterial` _trafficlightgreenstartb1 (`self.GreenTrafficLight`) "/Game/PoliceAI/Materials/TrafficLightMaterials/M_DefaultMaterial.M_DefaultMaterial")
      (`PrimitiveComponent.SetMaterial` (`self.TrafficLightGreenStartB2`) (`self.GreenTrafficLight`) "/Game/PoliceAI/Materials/TrafficLightMaterials/M_DefaultMaterial.M_DefaultMaterial")
      (`PrimitiveComponent.SetMaterial` _trafficlightgreenstartb1 (`self.YellowTrafficLight`) _returnvalue)
      (`PrimitiveComponent.SetMaterial` (`self.TrafficLightGreenStartB2`) (`self.YellowTrafficLight`) _returnvalue)
      (`PrimitiveComponent.SetMaterial` (`self.TrafficLightGreenStartB2`) (`self.RedTrafficLight`) "/Game/PoliceAI/Materials/TrafficLightMaterials/M_DefaultMaterial.M_DefaultMaterial")
      (`PrimitiveComponent.SetMaterial` _trafficlightgreenstartb1 (`self.RedTrafficLight`) "/Game/PoliceAI/Materials/TrafficLightMaterials/M_DefaultMaterial.M_DefaultMaterial")
      (`MaterialInstanceDynamic.SetScalarParameterValue` _returnvalue "Emissive" 15.0))
    (:`then_1`
      (bind _returnvalue_2 (`KismetMaterialLibrary.CreateDynamicMaterialInstance` "/Game/PoliceAI/Materials/TrafficLightMaterials/MaterialInstances/MI_RedTrafficLight.MI_RedTrafficLight" "None"))
      (`PrimitiveComponent.SetMaterial` _trafficlightredstarta2 (`self.RedTrafficLight`) _returnvalue_2)
      (`PrimitiveComponent.SetMaterial` (`self.TrafficLightRedStartA1`) (`self.RedTrafficLight`) _returnvalue_2)
      (`PrimitiveComponent.SetMaterial` _trafficlightredstarta2 (`self.YellowTrafficLight`) "/Game/PoliceAI/Materials/TrafficLightMaterials/M_DefaultMaterial.M_DefaultMaterial")
      (`PrimitiveComponent.SetMaterial` (`self.TrafficLightRedStartA1`) (`self.YellowTrafficLight`) "/Game/PoliceAI/Materials/TrafficLightMaterials/M_DefaultMaterial.M_DefaultMaterial")
      (`PrimitiveComponent.SetMaterial` _trafficlightredstarta2 (`self.GreenTrafficLight`) "/Game/PoliceAI/Materials/TrafficLightMaterials/M_DefaultMaterial.M_DefaultMaterial")
      (`PrimitiveComponent.SetMaterial` (`self.TrafficLightRedStartA1`) (`self.GreenTrafficLight`) "/Game/PoliceAI/Materials/TrafficLightMaterials/M_DefaultMaterial.M_DefaultMaterial")
      (`MaterialInstanceDynamic.SetScalarParameterValue` _returnvalue_2 "Emissive" 15.0))))

(fn `LightSequence3`
  (bind _trafficlightgreenstartb2 (`self.TrafficLightGreenStartB2`))
  (bind _trafficlightredstarta2 (`self.TrafficLightRedStartA2`))
  ;[1 1 1] Light Sequence 3
  (`|ExecutionSequence`
    (:`then_0`
      (bind _returnvalue (`KismetMaterialLibrary.CreateDynamicMaterialInstance` "/Game/PoliceAI/Materials/TrafficLightMaterials/MaterialInstances/MI_YellowTrafficLight.MI_YellowTrafficLight" "None"))
      (`PrimitiveComponent.SetMaterial` _trafficlightredstarta2 (`self.GreenTrafficLight`) "/Game/PoliceAI/Materials/TrafficLightMaterials/M_DefaultMaterial.M_DefaultMaterial")
      (`PrimitiveComponent.SetMaterial` (`self.TrafficLightRedStartA1`) (`self.GreenTrafficLight`) "/Game/PoliceAI/Materials/TrafficLightMaterials/M_DefaultMaterial.M_DefaultMaterial")
      (`PrimitiveComponent.SetMaterial` (`self.TrafficLightRedStartA1`) (`self.YellowTrafficLight`) _returnvalue)
      (`PrimitiveComponent.SetMaterial` _trafficlightredstarta2 (`self.YellowTrafficLight`) _returnvalue)
      (`PrimitiveComponent.SetMaterial` _trafficlightredstarta2 (`self.RedTrafficLight`) "/Game/PoliceAI/Materials/TrafficLightMaterials/M_DefaultMaterial.M_DefaultMaterial")
      (`PrimitiveComponent.SetMaterial` (`self.TrafficLightRedStartA1`) (`self.RedTrafficLight`) "/Game/PoliceAI/Materials/TrafficLightMaterials/M_DefaultMaterial.M_DefaultMaterial")
      (`MaterialInstanceDynamic.SetScalarParameterValue` _returnvalue "Emissive" 15.0))
    (:`then_1`
      (bind _returnvalue_2 (`KismetMaterialLibrary.CreateDynamicMaterialInstance` "/Game/PoliceAI/Materials/TrafficLightMaterials/MaterialInstances/MI_RedTrafficLight.MI_RedTrafficLight" "None"))
      (`PrimitiveComponent.SetMaterial` _trafficlightgreenstartb2 (`self.RedTrafficLight`) _returnvalue_2)
      (`PrimitiveComponent.SetMaterial` (`self.TrafficLightGreenStartB1`) (`self.RedTrafficLight`) _returnvalue_2)
      (`PrimitiveComponent.SetMaterial` _trafficlightgreenstartb2 (`self.YellowTrafficLight`) "/Game/PoliceAI/Materials/TrafficLightMaterials/M_DefaultMaterial.M_DefaultMaterial")
      (`PrimitiveComponent.SetMaterial` (`self.TrafficLightGreenStartB1`) (`self.YellowTrafficLight`) "/Game/PoliceAI/Materials/TrafficLightMaterials/M_DefaultMaterial.M_DefaultMaterial")
      (`PrimitiveComponent.SetMaterial` _trafficlightgreenstartb2 (`self.GreenTrafficLight`) "/Game/PoliceAI/Materials/TrafficLightMaterials/M_DefaultMaterial.M_DefaultMaterial")
      (`PrimitiveComponent.SetMaterial` (`self.TrafficLightGreenStartB1`) (`self.GreenTrafficLight`) "/Game/PoliceAI/Materials/TrafficLightMaterials/M_DefaultMaterial.M_DefaultMaterial")
      (`MaterialInstanceDynamic.SetScalarParameterValue` _returnvalue_2 "Emissive" 15.0))
    (:`then_2`
      (`SceneComponent.SetVisibility` (`self.StopZoneSpawnLocationA2`) false false)
      (`SceneComponent.SetVisibility` (`self.StopZoneSpawnLocationA1`) false false)
      (`SceneComponent.SetVisibility` (`self.StopZoneSpawnLocationB1`) true false)
      (`SceneComponent.SetVisibility` (`self.StopZoneSpawnLocationB2`) true false)
      (`self.K2_DestroyActor` (`self.StopZoneA1`))
      (`self.K2_DestroyActor` (`self.StopZoneA2`))
      (bind _returnvalue_3 (`|SpawnActorFromClass` "/Game/PoliceAI/Blueprints/TrafficSystem/BP_TrafficLightStopZone.BP_TrafficLightStopZone_C" (`SceneComponent.K2_GetComponentToWorld` (`self.StopZoneSpawnLocationB1`)) "AlwaysSpawn" "OverrideRootScale" null null))
      (set `self.StopZoneB1` _returnvalue_3)
      (bind _returnvalue_4 (`|SpawnActorFromClass` "/Game/PoliceAI/Blueprints/TrafficSystem/BP_TrafficLightStopZone.BP_TrafficLightStopZone_C" (`SceneComponent.K2_GetComponentToWorld` (`self.StopZoneSpawnLocationB2`)) "AlwaysSpawn" "OverrideRootScale" null null))
      (set `self.StopZoneB2` _returnvalue_4)
      (set `self.FirstRunPassed?` true))))

(fn `LightSequence4`
  (bind _trafficlightgreenstartb2 (`self.TrafficLightGreenStartB2`))
  (bind _trafficlightredstarta2 (`self.TrafficLightRedStartA2`))
  ;[1 1 1] Light Sequence 4
  (`|ExecutionSequence`
    (:`then_0`
      (bind _returnvalue (`KismetMaterialLibrary.CreateDynamicMaterialInstance` "/Game/PoliceAI/Materials/TrafficLightMaterials/MaterialInstances/MI_GreenTrafficLight.MI_GreenTrafficLight" "None"))
      (`PrimitiveComponent.SetMaterial` _trafficlightredstarta2 (`self.GreenTrafficLight`) _returnvalue)
      (`PrimitiveComponent.SetMaterial` (`self.TrafficLightRedStartA1`) (`self.GreenTrafficLight`) _returnvalue)
      (`PrimitiveComponent.SetMaterial` (`self.TrafficLightRedStartA1`) (`self.YellowTrafficLight`) "/Game/PoliceAI/Materials/TrafficLightMaterials/M_DefaultMaterial.M_DefaultMaterial")
      (`PrimitiveComponent.SetMaterial` _trafficlightredstarta2 (`self.YellowTrafficLight`) "/Game/PoliceAI/Materials/TrafficLightMaterials/M_DefaultMaterial.M_DefaultMaterial")
      (`PrimitiveComponent.SetMaterial` _trafficlightredstarta2 (`self.RedTrafficLight`) "/Game/PoliceAI/Materials/TrafficLightMaterials/M_DefaultMaterial.M_DefaultMaterial")
      (`PrimitiveComponent.SetMaterial` (`self.TrafficLightRedStartA1`) (`self.RedTrafficLight`) "/Game/PoliceAI/Materials/TrafficLightMaterials/M_DefaultMaterial.M_DefaultMaterial")
      (`MaterialInstanceDynamic.SetScalarParameterValue` _returnvalue "Emissive" 15.0))
    (:`then_1`
      (bind _returnvalue_2 (`KismetMaterialLibrary.CreateDynamicMaterialInstance` "/Game/PoliceAI/Materials/TrafficLightMaterials/MaterialInstances/MI_RedTrafficLight.MI_RedTrafficLight" "None"))
      (`PrimitiveComponent.SetMaterial` _trafficlightgreenstartb2 (`self.RedTrafficLight`) _returnvalue_2)
      (`PrimitiveComponent.SetMaterial` (`self.TrafficLightGreenStartB1`) (`self.RedTrafficLight`) _returnvalue_2)
      (`PrimitiveComponent.SetMaterial` _trafficlightgreenstartb2 (`self.YellowTrafficLight`) "/Game/PoliceAI/Materials/TrafficLightMaterials/M_DefaultMaterial.M_DefaultMaterial")
      (`PrimitiveComponent.SetMaterial` (`self.TrafficLightGreenStartB1`) (`self.YellowTrafficLight`) "/Game/PoliceAI/Materials/TrafficLightMaterials/M_DefaultMaterial.M_DefaultMaterial")
      (`PrimitiveComponent.SetMaterial` _trafficlightgreenstartb2 (`self.GreenTrafficLight`) "/Game/PoliceAI/Materials/TrafficLightMaterials/M_DefaultMaterial.M_DefaultMaterial")
      (`PrimitiveComponent.SetMaterial` (`self.TrafficLightGreenStartB1`) (`self.GreenTrafficLight`) "/Game/PoliceAI/Materials/TrafficLightMaterials/M_DefaultMaterial.M_DefaultMaterial")
      (`MaterialInstanceDynamic.SetScalarParameterValue` _returnvalue_2 "Emissive" 15.0))))

(fn `LightSequence5`
  (bind _trafficlightgreenstartb2 (`self.TrafficLightGreenStartB2`))
  (bind _trafficlightredstarta2 (`self.TrafficLightRedStartA2`))
  ;[1 1 1] Light Sequence 5
  (`|ExecutionSequence`
    (:`then_0`
      (bind _returnvalue (`KismetMaterialLibrary.CreateDynamicMaterialInstance` "/Game/PoliceAI/Materials/TrafficLightMaterials/MaterialInstances/MI_YellowTrafficLight.MI_YellowTrafficLight" "None"))
      (`PrimitiveComponent.SetMaterial` _trafficlightredstarta2 (`self.GreenTrafficLight`) "/Game/PoliceAI/Materials/TrafficLightMaterials/M_DefaultMaterial.M_DefaultMaterial")
      (`PrimitiveComponent.SetMaterial` (`self.TrafficLightRedStartA1`) (`self.GreenTrafficLight`) "/Game/PoliceAI/Materials/TrafficLightMaterials/M_DefaultMaterial.M_DefaultMaterial")
      (`PrimitiveComponent.SetMaterial` (`self.TrafficLightRedStartA1`) (`self.YellowTrafficLight`) _returnvalue)
      (`PrimitiveComponent.SetMaterial` _trafficlightredstarta2 (`self.YellowTrafficLight`) _returnvalue)
      (`PrimitiveComponent.SetMaterial` _trafficlightredstarta2 (`self.RedTrafficLight`) "/Game/PoliceAI/Materials/TrafficLightMaterials/M_DefaultMaterial.M_DefaultMaterial")
      (`PrimitiveComponent.SetMaterial` (`self.TrafficLightRedStartA1`) (`self.RedTrafficLight`) "/Game/PoliceAI/Materials/TrafficLightMaterials/M_DefaultMaterial.M_DefaultMaterial")
      (`MaterialInstanceDynamic.SetScalarParameterValue` _returnvalue "Emissive" 15.0))
    (:`then_1`
      (bind _returnvalue_2 (`KismetMaterialLibrary.CreateDynamicMaterialInstance` "/Game/PoliceAI/Materials/TrafficLightMaterials/MaterialInstances/MI_RedTrafficLight.MI_RedTrafficLight" "None"))
      (`PrimitiveComponent.SetMaterial` _trafficlightgreenstartb2 (`self.RedTrafficLight`) _returnvalue_2)
      (`PrimitiveComponent.SetMaterial` (`self.TrafficLightGreenStartB1`) (`self.RedTrafficLight`) _returnvalue_2)
      (`PrimitiveComponent.SetMaterial` _trafficlightgreenstartb2 (`self.YellowTrafficLight`) "/Game/PoliceAI/Materials/TrafficLightMaterials/M_DefaultMaterial.M_DefaultMaterial")
      (`PrimitiveComponent.SetMaterial` (`self.TrafficLightGreenStartB1`) (`self.YellowTrafficLight`) "/Game/PoliceAI/Materials/TrafficLightMaterials/M_DefaultMaterial.M_DefaultMaterial")
      (`PrimitiveComponent.SetMaterial` _trafficlightgreenstartb2 (`self.GreenTrafficLight`) "/Game/PoliceAI/Materials/TrafficLightMaterials/M_DefaultMaterial.M_DefaultMaterial")
      (`PrimitiveComponent.SetMaterial` (`self.TrafficLightGreenStartB1`) (`self.GreenTrafficLight`) "/Game/PoliceAI/Materials/TrafficLightMaterials/M_DefaultMaterial.M_DefaultMaterial")
      (`MaterialInstanceDynamic.SetScalarParameterValue` _returnvalue_2 "Emissive" 15.0))))

(fn `LightSequence6`
  (bind _trafficlightgreenstartb1 (`self.TrafficLightGreenStartB1`))
  (bind _trafficlightredstarta2 (`self.TrafficLightRedStartA2`))
  ;[1 1 1] Light Sequence 6
  (`|ExecutionSequence`
    (:`then_0`
      (bind _returnvalue (`KismetMaterialLibrary.CreateDynamicMaterialInstance` "/Game/PoliceAI/Materials/TrafficLightMaterials/MaterialInstances/MI_YellowTrafficLight.MI_YellowTrafficLight" "None"))
      (`PrimitiveComponent.SetMaterial` _trafficlightgreenstartb1 (`self.GreenTrafficLight`) "/Game/PoliceAI/Materials/TrafficLightMaterials/M_DefaultMaterial.M_DefaultMaterial")
      (`PrimitiveComponent.SetMaterial` (`self.TrafficLightGreenStartB2`) (`self.GreenTrafficLight`) "/Game/PoliceAI/Materials/TrafficLightMaterials/M_DefaultMaterial.M_DefaultMaterial")
      (`PrimitiveComponent.SetMaterial` _trafficlightgreenstartb1 (`self.YellowTrafficLight`) _returnvalue)
      (`PrimitiveComponent.SetMaterial` (`self.TrafficLightGreenStartB2`) (`self.YellowTrafficLight`) _returnvalue)
      (`PrimitiveComponent.SetMaterial` (`self.TrafficLightGreenStartB2`) (`self.RedTrafficLight`) "/Game/PoliceAI/Materials/TrafficLightMaterials/M_DefaultMaterial.M_DefaultMaterial")
      (`PrimitiveComponent.SetMaterial` _trafficlightgreenstartb1 (`self.RedTrafficLight`) "/Game/PoliceAI/Materials/TrafficLightMaterials/M_DefaultMaterial.M_DefaultMaterial")
      (`MaterialInstanceDynamic.SetScalarParameterValue` _returnvalue "Emissive" 15.0))
    (:`then_1`
      (bind _returnvalue_2 (`KismetMaterialLibrary.CreateDynamicMaterialInstance` "/Game/PoliceAI/Materials/TrafficLightMaterials/MaterialInstances/MI_RedTrafficLight.MI_RedTrafficLight" "None"))
      (`PrimitiveComponent.SetMaterial` _trafficlightredstarta2 (`self.RedTrafficLight`) _returnvalue_2)
      (`PrimitiveComponent.SetMaterial` (`self.TrafficLightRedStartA1`) (`self.RedTrafficLight`) _returnvalue_2)
      (`PrimitiveComponent.SetMaterial` _trafficlightredstarta2 (`self.YellowTrafficLight`) "/Game/PoliceAI/Materials/TrafficLightMaterials/M_DefaultMaterial.M_DefaultMaterial")
      (`PrimitiveComponent.SetMaterial` (`self.TrafficLightRedStartA1`) (`self.YellowTrafficLight`) "/Game/PoliceAI/Materials/TrafficLightMaterials/M_DefaultMaterial.M_DefaultMaterial")
      (`PrimitiveComponent.SetMaterial` _trafficlightredstarta2 (`self.GreenTrafficLight`) "/Game/PoliceAI/Materials/TrafficLightMaterials/M_DefaultMaterial.M_DefaultMaterial")
      (`PrimitiveComponent.SetMaterial` (`self.TrafficLightRedStartA1`) (`self.GreenTrafficLight`) "/Game/PoliceAI/Materials/TrafficLightMaterials/M_DefaultMaterial.M_DefaultMaterial")
      (`MaterialInstanceDynamic.SetScalarParameterValue` _returnvalue_2 "Emissive" 15.0))
    (:`then_2`
      (`SceneComponent.SetVisibility` (`self.StopZoneSpawnLocationA2`) true false)
      (`SceneComponent.SetVisibility` (`self.StopZoneSpawnLocationA1`) true false)
      (bind _returnvalue_3 (`|SpawnActorFromClass` "/Game/PoliceAI/Blueprints/TrafficSystem/BP_TrafficLightStopZone.BP_TrafficLightStopZone_C" (`SceneComponent.K2_GetComponentToWorld` (`self.StopZoneSpawnLocationA1`)) "AlwaysSpawn" "OverrideRootScale" null null))
      (set `self.StopZoneA1` _returnvalue_3)
      (bind _returnvalue_4 (`|SpawnActorFromClass` "/Game/PoliceAI/Blueprints/TrafficSystem/BP_TrafficLightStopZone.BP_TrafficLightStopZone_C" (`SceneComponent.K2_GetComponentToWorld` (`self.StopZoneSpawnLocationA2`)) "AlwaysSpawn" "OverrideRootScale" null null))
      (set `self.StopZoneA2` _returnvalue_4)
      (`SceneComponent.SetVisibility` (`self.StopZoneSpawnLocationB2`) false false)
      (`SceneComponent.SetVisibility` (`self.StopZoneSpawnLocationB1`) false false)
      (if (`self.FirstRunPassed?`)
        (`self.K2_DestroyActor` (`self.StopZoneB1`))
        (`self.K2_DestroyActor` (`self.StopZoneB2`))))))

(fn `PreContruct`
  ;[1 1 1] Default Light Setting Before Sequence Start
  (`SceneComponent.SetVisibility` (`self.StopZoneSpawnLocationA2`) true false)
  (`SceneComponent.SetVisibility` (`self.StopZoneSpawnLocationA1`) true false)
  (bind _returnvalue (`|SpawnActorFromClass` "/Game/PoliceAI/Blueprints/TrafficSystem/BP_TrafficLightStopZone.BP_TrafficLightStopZone_C" (`SceneComponent.K2_GetComponentToWorld` (`self.StopZoneSpawnLocationA1`)) "AlwaysSpawn" "OverrideRootScale" null null))
  (set `self.StopZoneA1` _returnvalue)
  (bind _returnvalue_2 (`|SpawnActorFromClass` "/Game/PoliceAI/Blueprints/TrafficSystem/BP_TrafficLightStopZone.BP_TrafficLightStopZone_C" (`SceneComponent.K2_GetComponentToWorld` (`self.StopZoneSpawnLocationA2`)) "AlwaysSpawn" "OverrideRootScale" null null))
  (set `self.StopZoneA2` _returnvalue_2)
  (`SceneComponent.SetVisibility` (`self.StopZoneSpawnLocationB2`) false false)
  (`SceneComponent.SetVisibility` (`self.StopZoneSpawnLocationB1`) false false)
  (if (`self.FirstRunPassed?`)
    (`self.K2_DestroyActor` (`self.StopZoneB1`))
    (`self.K2_DestroyActor` (`self.StopZoneB2`))))

(fn `UserConstructionScript`)