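; BP_Object_Pawn is a pawn that builds a block of instanced mesh copies in its Construction Script.
; Nested loops over Length, Width and Height add local-space instances to one InstancedStaticMesh, gridded by Spacing on X and Z.
; Y is random within a single Spacing, so the Width loop only stacks more instances into that thin slab; its computed offset is unconnected.
; The event graph has no gameplay logic.
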(event `self.ReceiveBeginPlay`)

(fn `UserConstructionScript`
  (bind _spacing (`self.Spacing`))
  (for _index (range (+ (`self.Length`) 1))
    (for _index_2 (range (+ (`self.Width`) 1))
      (for _index_3 (range (+ (`self.Height`) 1))
        (`InstancedStaticMeshComponent.AddInstance` (`self.InstancedStaticMesh`) (`KismetMathLibrary.MakeTransform` (`KismetMathLibrary.MakeVector` (`KismetMathLibrary.Conv_IntToDouble` (* _index _spacing)) (* _spacing (`KismetMathLibrary.RandomFloatInRange` 0.0 1.0)) (`KismetMathLibrary.Conv_IntToDouble` (* _index_3 _spacing)))) false)))))