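; Digital clock actor for the Spa track that displays the time of a BP_StylizedSky.
; Tick formats the sky's clock time into a 'Current Time' am/pm text, and BeginPlay resets the sky to time zero when AutoRun is set.
; The construction script fills hour, minute and second texts from the parent sky, passing system-time values as GetClockTime's day-length parameters.
; Its own time-setting functions are stubs or only call stubs.
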(event `self.ReceiveBeginPlay`
  (bind _stylized_sky (`self.Stylized Sky`))
  (if (`self.AutoRun?`)
    (`/Engine/EditorBlueprintResources/StandardMacros.IsValid` _stylized_sky
      (:`Is Valid`
        (`/Game/SoStylized/Environment/Sky/BP_StylizedSky.Set Time` _stylized_sky 0.0)))))

(event `self.ReceiveTick`
  (params (DeltaSeconds :type "Float (single-precision)"))
  (bind _stylized_sky (`self.Stylized Sky`))
  (bind (_hour _minute _second _pm_) (`/Game/SoStylized/Environment/Sky/BP_StylizedSky.Get Clock Time` _stylized_sky 24.0 60.0 60.0 false))
  (`/Engine/EditorBlueprintResources/StandardMacros.IsValid` _stylized_sky
    (:`Is Valid`
      (`TextRenderComponent.K2_SetText` (`self.CurrentTimeText`) (`|FormatText` "Current Time: {hh}:{mm}:{ss}{period}" _hour _minute _second (select `bool` _pm_ :`false` "am" :`true` "pm"))))))

(fn `ClockTimeToSkyTime`
  (params (`New Hours` :type "Float (double-precision)") (`New Minutes` :type "Float (double-precision)") (`Daily Hours` :type "Float (double-precision)") (`Hourly Minutes` :type "Float (double-precision)"))
  (returns (`Sky Time` :type "Float (double-precision)"))
  (return 0.0))

(fn `Set Time`
  (params (`New Time` :type "Float (double-precision)")))

(fn `Set Time ClockBased`
  (params (NewHour :type "Float (double-precision)") (NewMinutes :type "Float (double-precision)") (`Daily Hours` :type "Float (double-precision)" :default 24.0) (`Hourly Minutes` :type "Float (double-precision)" :default 60.0))
  (bind _sky_time (`self.ClockTimeToSkyTime` NewHour NewMinutes `Daily Hours` `Hourly Minutes`))
  (`self.Set Time` _sky_time))

(fn `UserConstructionScript`
  (bind (_returnvalue_year _returnvalue_month _returnvalue_day _returnvalue_hour _returnvalue_minute _returnvalue_second) (`KismetMathLibrary.BreakDateTime` (`KismetMathLibrary.Now`)))
  (bind _asbp_stylized_sky (cast `/Game/SoStylized/Environment/Sky/BP_StylizedSky` (`self.GetParentActor`)))
  (bind (_hour _minute _second) (`/Game/SoStylized/Environment/Sky/BP_StylizedSky.Get Clock Time` _asbp_stylized_sky (`KismetMathLibrary.Conv_IntToDouble` _returnvalue_hour) (`KismetMathLibrary.Conv_IntToDouble` _returnvalue_minute) (`KismetMathLibrary.Conv_IntToDouble` _returnvalue_second) false))
  (`TextRenderComponent.K2_SetText` (`self.Current Hour`) (`KismetTextLibrary.Conv_StringToText` _hour))
  (`TextRenderComponent.K2_SetText` (`self.Current Minute`) (`KismetTextLibrary.Conv_StringToText` _minute))
  (`TextRenderComponent.K2_SetText` (`self.Current Second`) (`KismetTextLibrary.Conv_StringToText` _second)))