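; Billboard clock on the Montreal track that shows the in-game time of day on two sets of hour and minute hands.
; BeginPlay caches the Ultra Dynamic Sky actor, whose TimeOfDay is wrapped and mapped to hand pitch, 1200 units per hour-hand turn and 100 per minute-hand turn.
; The second set of hands uses negated rotations.
; Tick enters a self-looping one-second Delay that refreshes the rotations.
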(event `self.ReceiveBeginPlay`
  (bind _returnvalue (`GameplayStatics.GetActorOfClass` "/Game/UltraDynamicSky/Blueprints/Ultra_Dynamic_Sky.Ultra_Dynamic_Sky_C"))
  (set `self.UDS` _returnvalue))

(event `self.ReceiveTick`
  (params (DeltaSeconds :type "Float (single-precision)"))
  (bind _returnvalue (`KismetMathLibrary.MakeRotator` 0.0 (`KismetMathLibrary.MapRangeClamped` (mod (`/Game/UltraDynamicSky/Blueprints/Ultra_Dynamic_Sky.Time of Day` (`self.UDS`)) 100.0) 0.0 100.0 0.0 360.0)))
  (bind _returnvalue_2 (`KismetMathLibrary.MakeRotator` 0.0 (`KismetMathLibrary.MapRangeClamped` (mod (`/Game/UltraDynamicSky/Blueprints/Ultra_Dynamic_Sky.Time of Day` (`self.UDS`)) 1200.0) 0.0 1200.0 0.0 360.0)))
  (`SceneComponent.K2_SetRelativeRotation` (`self.SM_Clock_HourHand_002`) _returnvalue_2 false false :!label _label)
  (`SceneComponent.K2_SetRelativeRotation` (`self.SM_Clock_HourHand_001`) (`KismetMathLibrary.NegateRotator` _returnvalue_2) false false)
  (`SceneComponent.K2_SetRelativeRotation` (`self.SM_Clock_MinuterHand_002`) _returnvalue false false)
  (`SceneComponent.K2_SetRelativeRotation` (`self.SM_Clock_MinuterHand_001`) (`KismetMathLibrary.NegateRotator` _returnvalue) false false)
  (`KismetSystemLibrary.Delay` 1.0)
  (goto _label))

(fn `UserConstructionScript`)