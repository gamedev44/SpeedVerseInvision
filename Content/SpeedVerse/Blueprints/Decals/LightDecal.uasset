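; LightDecal is a decal actor with a configurable material and size, set up entirely in the Construction Script; its event graph is empty.
; The script multiplies the Decal component's world scale by a fixed depth factor plus Height and Width, then applies NewDecalMaterial.
; ProportionalScalingLocked copies Width into Height, but only after the scale has been applied.
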(fn `UserConstructionScript`
  (`SceneComponent.SetWorldScale3D` (`self.Decal`) (* (`SceneComponent.K2_GetComponentScale` (`self.Decal`)) (`KismetMathLibrary.MakeVector` 0.2 (`self.Height`) (`self.Width`))))
  (`DecalComponent.SetDecalMaterial` (`self.Decal`) (`self.New Decal Material`))
  (if (`self.Proportional Scaling Locked`)
    (set `self.Height` (`self.Width`))
    (set `self.Width` (`self.Height`))
    (else
      (set `self.Height` (`self.Height`))
      (set `self.Width` (`self.Height`)))))